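; BP_BorderGrass01 is a construction-time tool that scatters grass along a spline as hierarchical instanced static meshes.
; Unless BuildingMode is on, it adds instances at DistanceBetween intervals, randomizing position along and beside the spline, yaw and uniform scale.
; Instance rotation follows the spline, with an added roll offset.
; Cull distance derives from the MPC_Grass Distance parameter plus a fixed margin.
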(fn `UserConstructionScript`
  (if (not (`self.BuildingMode?`))
    (bind _returnvalue (`KismetMaterialLibrary.GetScalarParameterValue` "/Game/PirateIsland/Include/Materials/Collections/MPC_Grass.MPC_Grass" "Distance"))
    (`PrimitiveComponent.SetCullDistance` (`self.HierarchicalInstancedStaticMesh`) (+ _returnvalue 1200.0))
    (for _index (range (+ (`KismetMathLibrary.FTrunc` (/ (`SplineComponent.GetSplineLength` (`self.Spline`)) (`self.DistanceBetween`))) 1))
      (bind _returnvalue_2 (+ (* _index (`self.DistanceBetween`)) (`KismetMathLibrary.RandomFloatInRange` (* (`self.RighLeftVariation`) -1.0) (`self.RighLeftVariation`))))
      (bind (_returnvalue_roll _returnvalue_pitch _returnvalue_yaw) (`KismetMathLibrary.BreakRotator` (`SplineComponent.GetRotationAtDistanceAlongSpline` (`self.Spline`) _returnvalue_2 "Local")))
      (`InstancedStaticMeshComponent.AddInstance` (`self.HierarchicalInstancedStaticMesh`) (`KismetMathLibrary.MakeTransform` (+ (`SplineComponent.GetLocationAtDistanceAlongSpline` (`self.Spline`) _returnvalue_2 "Local") (* (`SplineComponent.GetRightVectorAtDistanceAlongSpline` (`self.Spline`) _returnvalue_2 "Local") (`KismetMathLibrary.RandomFloatInRange` (`self.FrontMin`) (`self.FrontMax`)))) (`KismetMathLibrary.MakeRotator` (+ _returnvalue_roll (`self.Roll`)) _returnvalue_pitch (+ _returnvalue_yaw (`KismetMathLibrary.RandomFloatInRange` (`self.YawMin`) (`self.YawMax`)))) (`KismetMathLibrary.Conv_DoubleToVector` (`KismetMathLibrary.RandomFloatInRange` (`self.ScaleMin`) (`self.ScaleMax`))))))))