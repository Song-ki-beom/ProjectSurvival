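; BP_OceanManager drives the ocean's wave settings and calculates water surface height on the CPU.
; On construction and BeginPlay, it writes wave parameters and the ocean mesh actor's height into MPC_Weather, warning if no mesh is assigned.
; FGetWaveHeight reads wind/wave Direction from that collection and sums three time-based Gerstner waves at the stored Location, scaled and angled from one base wave, plus surface height and an offset.
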(event `CE_BeginPlay`
  (`self.F_SetParameters` :!label _label))

(event `self.ReceiveBeginPlay`
  (goto _label))

(fn `F_GerstnerWave`
  (params (WaveLength :type "Float (double-precision)" :default 4000.0) (Steps :type "Float (double-precision)" :default 2.0) (Amplitude :type "Float (double-precision)" :default 30.0) (Direction :type "Vector Structure"))
  (returns (Displace :type "Vector Structure"))
  (bind _returnvalue (* Steps Amplitude))
  (bind _returnvalue_2 (/ 2.0 (/ WaveLength (`KismetMathLibrary.MultiplyByPi` 2.0))))
  (bind _returnvalue_3 (+ (`KismetMathLibrary.Dot_VectorVector` (* (* Direction (1.0 1.0 0.0)) _returnvalue_2) (* (`self.Location`) (1.0 1.0 0.0))) (* (* (* (`KismetMathLibrary.Sqrt` (* (/ 6.3 WaveLength) 9.8)) WaveLength) _returnvalue_2) (`KismetSystemLibrary.GetGameTimeInSeconds`))))
  (bind _returnvalue_4 (`KismetMathLibrary.Cos` _returnvalue_3))
  (return (`KismetMathLibrary.MakeVector` (* (* _returnvalue (.x Direction)) _returnvalue_4) (* _returnvalue_4 (* _returnvalue (.y Direction))) (* (`KismetMathLibrary.Sin` _returnvalue_3) Amplitude))))

(fn `F_GetWaveHeight`
  (params (Location :type "Vector Structure") (SurfaceZOffset :type "Float (double-precision)" :default -20.0))
  (returns (Height :type "Float (double-precision)"))
  (bind (_directionadd_x _directionadd_y) (`KismetMathLibrary.BreakVector` (`self.DirectionAdd`)))
  (bind (_direction_r _direction_g) (break `LinearColor` (`self.Direction`)))
  (bind (_directionadd_x_2 _directionadd_y_2) (`KismetMathLibrary.BreakVector` (`self.DirectionAdd`)))
  (bind (_direction_r_2 _direction_g_2) (break `LinearColor` (`self.Direction`)))
  (bind (_direction_r_3 _direction_g_3) (break `LinearColor` (`self.Direction`)))
  (set `self.Location` (`KismetMathLibrary.MakeVector` Location_X Location_Y (`self.SurfaceZ`)))
  ;[1 1 1] Direction
  (bind _returnvalue (`KismetMaterialLibrary.GetVectorParameterValue` "/Game/PirateIsland/Include/Materials/Collections/MPC_Weather.MPC_Weather" "Direction"))
  (set `self.Direction` _returnvalue)
  (`|ExecutionSequence`
    (:`then_0`
      ;[1 1 1] GerstnerWave
      (bind _displace (`self.F_GerstnerWave` (`self.Length01`) (`self.Steps01`) (`self.Amplitude01`) (`KismetMathLibrary.MakeVector` _direction_r_3 _direction_g_3)))
      (set `self.Z01` (.z _displace)))
    (:`then_1`
      (bind _displace_2 (`self.F_GerstnerWave` (* (`self.Length01`) 0.75) (* (`self.Steps01`) 1.75) (* (`self.Amplitude01`) 0.75) (`KismetMathLibrary.MakeVector` (- _direction_r_2 _directionadd_x) (- _direction_g_2 _directionadd_y))))
      (set `self.Z02` (.z _displace_2)))
    (:`then_2`
      (bind _displace_3 (`self.F_GerstnerWave` (* (`self.Length01`) 0.5) (* (`self.Steps01`) 0.33) (* (`self.Amplitude01`) 0.5) (`KismetMathLibrary.MakeVector` (+ _directionadd_x_2 _direction_r) (+ _directionadd_y_2 _direction_g))))
      (return (+ (`self.SurfaceZ`) (+ (`self.Z01`) (`self.Z02`) (.z _displace_3)) SurfaceZOffset)))))

(fn `F_SetParameters`
  (bind _oceanmeshactor (`self.OceanMeshActor`))
  (bind (_returnvalue_x _returnvalue_y _returnvalue_z) (`KismetMathLibrary.BreakVector` (`self.K2_GetActorLocation` _oceanmeshactor)))
  ;[1 1 1] Wave
  (`KismetMaterialLibrary.SetScalarParameterValue` "/Game/PirateIsland/Include/Materials/Collections/MPC_Weather.MPC_Weather" "Amplitude" (`self.Amplitude01`))
  (`KismetMaterialLibrary.SetScalarParameterValue` "/Game/PirateIsland/Include/Materials/Collections/MPC_Weather.MPC_Weather" "Length" (`self.Length01`))
  (`KismetMaterialLibrary.SetScalarParameterValue` "/Game/PirateIsland/Include/Materials/Collections/MPC_Weather.MPC_Weather" "Steps" (`self.Steps01`))
  (`KismetMaterialLibrary.SetVectorParameterValue` "/Game/PirateIsland/Include/Materials/Collections/MPC_Weather.MPC_Weather" "DirectionAdd" (`KismetMathLibrary.Conv_VectorToLinearColor` (`self.DirectionAdd`)))
  (`/Engine/EditorBlueprintResources/StandardMacros.IsValid` _oceanmeshactor
    (:`Is Valid`
      (`KismetMaterialLibrary.SetScalarParameterValue` "/Game/PirateIsland/Include/Materials/Collections/MPC_Weather.MPC_Weather" "WaterHeight" _returnvalue_z)
      ;[1 1 1] GetSurfaceZ
      (set `self.SurfaceZ` _returnvalue_z))
    (:`Is Not Valid`
      (`KismetSystemLibrary.PrintString` "No OceanMesh selected in OceanManager" true true (struct :`R` 1.0 :`G` 0.390872 :`A` 1.0) 4.0))))

(fn `UserConstructionScript`
  (`self.CE_BeginPlay`))