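; BP_WeatherManager is a weather actor that pushes global wind settings into the MPC_Weather material parameter collection.
; Its FSetParameters function writes the Speed and Wind scalars and uses the actor's forward vector as the Direction vector, so rotating the actor sets the direction.
; It also caches that direction and its yaw in variables.
; The function runs from both the construction script and BeginPlay, with no per-frame updates.
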(event `self.ReceiveBeginPlay`
  (`self.F_SetParameters`))

(fn `F_SetParameters`
  (bind _returnvalue (`KismetMathLibrary.Conv_VectorToLinearColor` (`self.GetActorForwardVector`)))
  (`KismetMaterialLibrary.SetScalarParameterValue` "/Game/PirateIsland/Include/Materials/Collections/MPC_Weather.MPC_Weather" "Speed" (`self.Speed`))
  (`KismetMaterialLibrary.SetScalarParameterValue` "/Game/PirateIsland/Include/Materials/Collections/MPC_Weather.MPC_Weather" "Wind" (`self.Wind`))
  (`KismetMaterialLibrary.SetVectorParameterValue` "/Game/PirateIsland/Include/Materials/Collections/MPC_Weather.MPC_Weather" "Direction" _returnvalue)
  (bind _output_get (set `self.Direction` _returnvalue))
  (set `self.Yaw` (.yaw (`KismetMathLibrary.Conv_VectorToRotator` (`KismetMathLibrary.Conv_LinearColorToVector` _output_get)))))

(fn `UserConstructionScript`
  (`self.F_SetParameters`))