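; Buoyant prop actor that floats a configurable mesh on waves from BP_OceanManager, auto-found at construction unless selected manually.
; With physics, an upward force scales with depth below the sampled wave height; otherwise, the mesh snaps to that height.
; Optional surface tilt comes from forward and side wave samples.
; Camera distance drives optimization, switching physics to simple snapping and lengthening the tick interval.
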(event `self.ReceiveBeginPlay`
  (`KismetSystemLibrary.Delay` (`self.DelayToStartSimulate`))
  (`PrimitiveComponent.SetSimulatePhysics` (`self.SM_Barrel01`) (`self.PhysicSimulation?`))
  (`self.CE_SimulationBegin`))

(event `self.ReceiveTick`
  (params (DeltaSeconds :type "Float (single-precision)"))
  (bind _currentheight (`self.CurrentHeight`))
  (bind _returnvalue (`SceneComponent.K2_GetComponentLocation` (`self.SM_Barrel01`)))
  (bind _returnvalue_2 (`SceneComponent.K2_GetComponentLocation` (`self.SM_Barrel01`)))
  (bind (_returnvalue_x _returnvalue_y _returnvalue_z) (`KismetMathLibrary.BreakVector` (`SceneComponent.K2_GetComponentLocation` (`self.SM_Barrel01`))))
  ;[1 1 1] LODs Switcher
  (`self.F_Optimization`)
  (`/Engine/EditorBlueprintResources/StandardMacros.IsValid` (`self.OceanManager`)
    (:`Is Valid`
      (if (`SceneComponent.IsSimulatingPhysics` (`self.SM_Barrel01`) "None")
        (if (`self.SimpleMovingOnDistance?`)
          ;[0 0.535 0.09056] Physical to Simple and Revert. Optimization
          (`|ExecutionSequence`
            (:`then_0`
              (`/Engine/EditorBlueprintResources/StandardMacros.Gate` true :!label _label
                (:`Exit`
                  (`/Engine/EditorBlueprintResources/StandardMacros.DoOnce` false :!label _label_2
                    (:`Completed`
                      (`|ExecutionSequence`
                        (:`then_0`
                          (`self.K2_SetActorLocation` _returnvalue)
                          (`PrimitiveComponent.SetSimulatePhysics` (`self.SM_Barrel01`) false))
                        (:`then_1`
                          (goto _label_6 :!via `Reset`))))))))
            (:`then_1`
              ;[0.02987 0.311 0.51] Simple Simulation
              (bind _height (`/Game/PirateIsland/Include/Blueprints/Water/BP_OceanManager.F_GetWaveHeight` (`self.OceanManager`) _returnvalue_2 (`self.SurfaceZOffset`) :!label _label_3))
              (set `self.CurrentHeight` _height)
              (`SceneComponent.K2_SetWorldLocation` (`self.SM_Barrel01`) (`KismetMathLibrary.MakeVector` (.x _returnvalue_2) (.y _returnvalue_2) (`self.CurrentHeight`)) false false)
              ;[0.175 0.2839 1] RotateToSurface
              (if (`self.RotateToSurface?`) :!label _label_4
                (`self.F_RotateToSurface`))))
          (else
            (`|ExecutionSequence`
              (:`then_0`
                (`/Engine/EditorBlueprintResources/StandardMacros.Gate` true :!label _label_5
                  (:`Exit`
                    (`/Engine/EditorBlueprintResources/StandardMacros.DoOnce` false :!label _label_6
                      (:`Completed`
                        (`|ExecutionSequence`
                          (:`then_0`
                            (`self.K2_SetActorLocation` _returnvalue)
                            (`PrimitiveComponent.SetSimulatePhysics` (`self.SM_Barrel01`) true))
                          (:`then_1`
                            (goto _label_2 :!via `Reset`))))))))
              (:`then_1`
                ;[1 0.5279 0.3049] Water Gravity Force
                (bind _height_2 (`/Game/PirateIsland/Include/Blueprints/Water/BP_OceanManager.F_GetWaveHeight` (`self.OceanManager`) (`SceneComponent.K2_GetComponentLocation` (`self.SM_Barrel01`)) (`self.SurfaceZOffset`)))
                (set `self.CurrentHeight` _height_2)
                (`PrimitiveComponent.AddForce` (`self.SM_Barrel01`) (* (0.0 0.0 1.0) (`KismetMathLibrary.MakeVector` 0.0 0.0 (* (`KismetMathLibrary.Abs` (- (`KismetMathLibrary.FClamp` _returnvalue_z 0.0 _currentheight) _currentheight)) (`self.Bounce`)))) "None" true)
                (goto _label_4)))))
        (else
          (goto _label_3))))))

(event `CE_SimulationBegin`
  ;[0 0.535 0.09056] Physical to Simple and Revert. Optimization
  (`|ExecutionSequence`
    (:`then_0`
      (goto _label_5 :!via `Open`))
    (:`then_1`
      (goto _label :!via `Open`))))

(fn `F_Optimization`
  (`|ExecutionSequence`
    (:`then_0`
      ;[1 1 1] Physic
      (if (`KismetMathLibrary.NearlyEqual_FloatFloat` (`KismetMathLibrary.FClamp` (/ (`self.GetDistanceTo` (`GameplayStatics.GetPlayerCameraManager` 0) self) (`self.DistanceStart`))) 1.0 0.05)
        (set `self.SimpleMovingOnDistance?` true)
        (else
          (set `self.SimpleMovingOnDistance?` false))))
    (:`then_1`
      ;[1 1 1] NoPhysic
      (`self.SetActorTickInterval` (`KismetMathLibrary.Lerp` 0.0 0.5 (`KismetMathLibrary.FClamp` (/ (- (`self.GetDistanceTo` (`GameplayStatics.GetPlayerCameraManager` 0) self) (`self.DistanceStart`)) (`self.DistanceToStop`))))))))

(fn `F_RotateToSurface`
  (locals (XHeight :type "Float (double-precision)") (YHeight :type "Float (double-precision)"))
  (bind (_returnvalue_roll _returnvalue_pitch _returnvalue_yaw) (`KismetMathLibrary.BreakRotator` (`self.K2_GetActorRotation`)))
  (bind _sm_barrel01 (`self.SM_Barrel01`))
  (bind _sm_barrel01_2 (`self.SM_Barrel01`))
  (bind _detectdistance (`self.DetectDistance`))
  (bind _detectdistance_2 (`self.DetectDistance`))
  (bind _intensity (`self.Intensity`))
  (`|ExecutionSequence`
    (:`then_0`
      (bind _height (`/Game/PirateIsland/Include/Blueprints/Water/BP_OceanManager.F_GetWaveHeight` (`self.OceanManager`) (+ (`SceneComponent.K2_GetComponentLocation` _sm_barrel01_2) (* (`SceneComponent.GetForwardVector` _sm_barrel01_2) (`KismetMathLibrary.MakeVector` _detectdistance _detectdistance))) (`self.SurfaceZOffset`)))
      (set `local.XHeight` _height))
    (:`then_1`
      (bind _height_2 (`/Game/PirateIsland/Include/Blueprints/Water/BP_OceanManager.F_GetWaveHeight` (`self.OceanManager`) (+ (`SceneComponent.K2_GetComponentLocation` _sm_barrel01) (* (`SceneComponent.GetRightVector` _sm_barrel01) (`KismetMathLibrary.MakeVector` _detectdistance_2 _detectdistance_2) (-1.0 -1.0 0.0))) (`self.SurfaceZOffset`)))
      (set `local.YHeight` _height_2))
    (:`then_2`
      (`SceneComponent.K2_SetRelativeRotation` (`self.SM_Barrel01`) (`KismetMathLibrary.MakeRotator` (* (- (`local.YHeight`) (`self.CurrentHeight`)) _intensity) (* (- (`local.XHeight`) (`self.CurrentHeight`)) _intensity) _returnvalue_yaw) false false))))

(fn `UserConstructionScript`
  (`StaticMeshComponent.SetStaticMesh` (`self.SM_Barrel01`) (`self.Mesh`))
  (if (not (`self.SelectManual?`))
    (bind _outactors (`GameplayStatics.GetAllActorsOfClass` "/Game/PirateIsland/Include/Blueprints/Water/BP_OceanManager.BP_OceanManager_C"))
    (set `self.OceanManager` (`|GetArrayItem` _outactors))))