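; BP_CrackedGround01 is a construction-time prop that lays a cracked ground mesh along a spline with an adjustable emissive look.
; The construction script adds one spline mesh and bends it between the first two spline points using their locations and tangents.
; It creates base and translucent dynamic instances of MI_CrackedGround01, sets the emissive color on both and applies gradient power to the translucent one.
; The event graph has no active logic.
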(fn `UserConstructionScript`
  (bind (_location _tangent) (`SplineComponent.GetLocationAndTangentAtSplinePoint` (`self.Spline`) 1 "Local"))
  (bind (_location_2 _tangent_2) (`SplineComponent.GetLocationAndTangentAtSplinePoint` (`self.Spline`) 0 "Local"))
  (bind _returnvalue (`AddComponent|NODE_AddSplineMeshComponent-0`))
  (`|ExecutionSequence`
    (:`then_0`
      (`SplineMeshComponent.SetStartAndEnd` _returnvalue _location_2 _tangent_2 _location _tangent true))
    (:`then_1`
      (bind _returnvalue_2 (`PrimitiveComponent.CreateDynamicMaterialInstance` _returnvalue 0 "/Game/PirateIsland/Include/Materials/MI_CrackedGround01.MI_CrackedGround01" "None"))
      (set `self.DynMatBase` _returnvalue_2)
      (bind _returnvalue_3 (`PrimitiveComponent.CreateDynamicMaterialInstance` _returnvalue 1 "/Game/PirateIsland/Include/Materials/Translucent/MI_CrackedGround01.MI_CrackedGround01" "None"))
      (bind _output_get (set `self.DynMatTranslucent` _returnvalue_3))
      (`MaterialInstanceDynamic.SetVectorParameterValue` _output_get "EmissiveColor" (`self.Emissive`))
      (`MaterialInstanceDynamic.SetVectorParameterValue` (`self.DynMatBase`) "EmissiveColor" (`self.Emissive`))
      (`MaterialInstanceDynamic.SetScalarParameterValue` (`self.DynMatTranslucent`) "GradientPower" (`self.GradientPower`)))))