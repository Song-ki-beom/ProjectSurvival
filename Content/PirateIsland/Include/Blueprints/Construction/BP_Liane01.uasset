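; BP_Liane01 is a construction-time liana (vine) actor that bends a static mesh along a spline.
; Its construction script adds a single spline mesh component, assigns the Mesh variable and sets the cull distance from MaxDrawDistance.
; The mesh takes its start and end positions and tangents from the first two spline points in local space, so any further points are ignored.
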(fn `UserConstructionScript`
  (locals (CurrentSplineMesh :type "SplineMeshComponent Object Reference"))
  (bind (_location _tangent) (`SplineComponent.GetLocationAndTangentAtSplinePoint` (`self.Spline`) 1 "Local"))
  (bind (_location_2 _tangent_2) (`SplineComponent.GetLocationAndTangentAtSplinePoint` (`self.Spline`) 0 "Local"))
  (bind _returnvalue (`AddComponent|NODE_AddSplineMeshComponent-0`))
  (bind _output_get (set `local.CurrentSplineMesh` _returnvalue))
  (`StaticMeshComponent.SetStaticMesh` _output_get (`self.Mesh`))
  (`PrimitiveComponent.SetCullDistance` (`local.CurrentSplineMesh`) (`self.MaxDrawDistance`))
  (`SplineMeshComponent.SetStartAndEnd` (`local.CurrentSplineMesh`) _location_2 _tangent_2 _location _tangent true))